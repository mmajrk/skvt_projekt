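; Player controller for Skvt that lets the player switch control between the Pawns in the level.
; BeginPlay adds the default player-mappable Enhanced Input config to the local player subsystem.
; The swap input action possesses the Pawn returned by GetPawnToPosess, which takes the one after the controlled Pawn in GetAllActorsOfClass order and wraps to the first at the end.
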(event `self.ReceiveBeginPlay`
  (bind _returnvalue (pcsubsystem `EnhancedInputLocalPlayerSubsystem` self))
  (`/Engine/EditorBlueprintResources/StandardMacros.IsValid` _returnvalue
    (:`Is Valid`
      (`EnhancedInputSubsystemInterface.AddPlayerMappableConfig` _returnvalue "/Game/Skvt/Characters/Input/PMI_Default.PMI_Default" (struct)))))

(event `EnhancedInput|/Game/Skvt/Characters/Input/Actions/IA_Swap`
  (params (ActionValue :type Boolean) (ElapsedSeconds :type "Float (double-precision)") (TriggeredSeconds :type "Float (double-precision)") (InputAction :type "InputAction Object Reference" :default "/Game/Skvt/Characters/Input/Actions/IA_Swap.IA_Swap"))
  (:`Triggered`
    (bind _selected_pawn (`self.GetPawnToPosess`))
    (`self.Possess` _selected_pawn)))

(fn `GetPawnToPosess`
  (returns (`Selected Pawn` :type "Pawn Object Reference"))
  (bind _outactors (`GameplayStatics.GetAllActorsOfClass` "/Script/Engine.Pawn"))
  (bind _returnvalue (+ (`KismetArrayLibrary.Array_Find` _outactors (`self.K2_GetPawn`)) 1))
  (if (`KismetArrayLibrary.Array_IsValidIndex` _outactors _returnvalue)
    (return (`|GetArrayItem` _outactors _returnvalue))
    (else
      (return (`|GetArrayItem` _outactors)))))

(fn `UserConstructionScript`)